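; Shop stall actor that opens the shop menu when any actor overlaps it.
; OpenShopGUI clears existing widgets, creates and stores the ShopGUI widget, switches to UI-only input, pauses the game, shows the cursor, removes the HUD and flags the shop as open.
; AddHudToViewport creates, stores and displays a new HUD widget, but nothing in this Blueprint calls it.
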(event EventBeginPlay)

(event EventActorBeginOverlap
  (params (OtherActor :type Actor%20Object%20Reference))
  (CallFunction|OpenShopGUI))

(event EventTick
  (params (DeltaSeconds :type Float%20%28single-precision%29)))

(fn ConstructionScript)

(fn OpenShopGUI
  (Viewport|RemoveAllWidgets)
  ;[1 1 1] Create the shop GUI
  (bind _returnvalue (UserInterface|CreateWidget "/Game/UI/ShopGUI.ShopGUI_C"))
  ;[1 1 1] Set reference to shop GUI
  (bind _output_get (Variables|Default|SetShopMenuReference _returnvalue))
  (Input|SetInputModeUIOnly (Game|GetPlayerController 0) _output_get false)
  ;[1 1 1] Add the shop GUI to the viewport
  (UserInterface|Viewport|AddtoViewport _returnvalue 0)
  ;[1 1 1] Pause the game
  (Game|SetGamePaused true)
  ;[1 1 1] Show the mouse cursor
  (Variables|/Script/Engine.PlayerController|SetbShowMouseCursor (Game|GetPlayerController 0) true)
  ;[1 1 1] Remove the HUD from the viewport
  (Widget|RemovefromParent (Variables|Default|GetHUD%20reference))
  ;[1 1 1] Let the system know the shop GUI is open
  (Variables|Default|SetShopOpen true)
  (return))

(fn AddHudtoViewport
  ;[1 1 1] Add HUD to viewport
  (bind _returnvalue (UserInterface|CreateWidget "/Game/UI/HUD.HUD_C"))
  (bind _output_get (Variables|Default|SetHUD%20reference _returnvalue))
  (UserInterface|Viewport|AddtoViewport _output_get 0))